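; BP_WalkingGrimic is a Grimic pawn that walks along the points of an assigned spline in a repeating loop.
; BeginPlay caches the point count of TargetSpline and starts at the first point.
; Every Tick issues an AI MoveTo toward the current point's world location, advancing the index on success and wrapping to zero after the last.
; Debug strings print when the index wraps or a move fails.
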(event `self.ReceiveBeginPlay`
  (set `self.MaxPathPoint` (`SplineComponent.GetNumberOfSplinePoints` (`/Game/Dynamic/Grimics/BP_Spline.Spline` (`self.TargetSpline`))))
  (set `self.PathPoint` 0))

(event `self.ReceiveTick`
  (params (DeltaSeconds :type "Float (single-precision)"))
  (`|AIMoveTo` self (.location (`SplineComponent.GetTransformAtSplinePoint` (`/Game/Dynamic/Grimics/BP_Spline.Spline` (`self.TargetSpline`)) (`self.PathPoint`) "World" false)) null 10.0
    (:`OnSuccess`
      (bind _result (`/Engine/EditorBlueprintResources/StandardMacros.IncrementInt` (`self.PathPoint`))
        (:`  `
          (if (not (< _result (`self.MaxPathPoint`)))
            (set `self.PathPoint` 0)
            (`KismetSystemLibrary.PrintString` "Success")))))
    (:`OnFail`
      (`KismetSystemLibrary.PrintString` "Fail"))))

(fn `UserConstructionScript`)