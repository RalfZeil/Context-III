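; BP_Baby is an interactable baby actor, filed under the Droochsloot hidden Blueprints, whose crying can be silenced.
; Its Interact override stops the BabycryingCue audio, then defers to the parent interaction and returns that result.
; The event graph holds only disabled default nodes, and the construction script just calls its parent.
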(fn `Interact`
  (params (Interacter :type "/Game/Dynamic/Player/Blueprints/BP_FirstPersonCharacter Object Reference"))
  (returns (result :type Boolean))
  (`AudioComponent.Stop` (`self.baby-crying_Cue`))
  ;[1 1 1] Call Parent Interaction for Functionality
  (bind _result (`parent.Interact` null))
  (return _result))

(fn `UserConstructionScript`
  (`parent.UserConstructionScript`))