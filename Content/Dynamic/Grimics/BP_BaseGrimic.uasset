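; BP_BaseGrimic is a base Grimic actor that burns away visually and disappears when hidden.
; On BeginPlay it applies a dynamic M_Grimic material to its skeletal mesh and binds to its StartHidingGrimic dispatcher.
; HideGrimic fires that dispatcher and disables collision.
; The bound event runs a timeline driving the material's Burn parameter, with a leftover debug print, then hides the actor.
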(event `self.ReceiveBeginPlay`
  (bind _skeletalmesh (`self.SkeletalMesh`))
  (add `self.StartHidingGrimic` (delegate `Hide Grimics`))
  (bind _returnvalue (`PrimitiveComponent.CreateDynamicMaterialInstance` _skeletalmesh 0 "/Game/Dynamic/World/materials/Props/M_Grimic.M_Grimic" "None"))
  (`PrimitiveComponent.SetMaterial` _skeletalmesh 0 _returnvalue))

(event `Hide Grimics`
  (bind (_direction _alpha) (`Timeline|BurnGrimic`)
    (:`Update`
      (`MaterialInstanceDynamic.SetScalarParameterValue` (stale `self.ReceiveBeginPlay` _returnvalue) "Burn" _alpha)
      (`KismetSystemLibrary.PrintString` "Hello"))
    (:`Finished`
      (`self.SetActorHiddenInGame` true))))

(fn `HideGrimic`
  (`self.StartHidingGrimic`)
  (`self.SetActorEnableCollision` false))

(fn `UserConstructionScript`)