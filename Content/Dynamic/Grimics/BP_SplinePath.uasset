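; BP_SplinePath is an actor that moves a referenced actor, MovingActor, along its Path spline.
; On BeginPlay, StartMoving plays the MoveOverPath timeline, whose Alpha is interpolated from zero to the full spline length.
; Each update samples the world-space transform at that distance and applies its location and rotation to MovingActor.
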(event `self.ReceiveBeginPlay`
  (`self.Start Moving`))

(event `Start Moving`
  (bind (_direction _alpha) (`Timeline|MoveOverPath`)
    (:`Update`
      (`self.K2_SetActorLocationAndRotation` (`self.MovingActor`) (.location (`SplineComponent.GetTransformAtDistanceAlongSpline` (`self.Path`) (`KismetMathLibrary.Lerp` 0.0 (`SplineComponent.GetSplineLength` (`self.Path`)) _alpha) "World" false)) (.rotation (`SplineComponent.GetTransformAtDistanceAlongSpline` (`self.Path`) (`KismetMathLibrary.Lerp` 0.0 (`SplineComponent.GetSplineLength` (`self.Path`)) _alpha) "World" false)) false false))))

(fn `UserConstructionScript`)