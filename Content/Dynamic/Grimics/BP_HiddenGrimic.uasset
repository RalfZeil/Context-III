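; BP_HiddenGrimic is a Grimic that hides behind a stand-in HiddenActor until that actor is interacted with.
; On BeginPlay it binds to the stand-in's interaction event and hides its own meshes and collision.
; That event swaps visibility and collision to reveal the Grimic and fires confetti Niagara.
; Interacting with the Grimic itself marks it caught and hides it, while ToggleInteractionGBP controls the stand-in's interactability.
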(event `self.ReceiveBeginPlay`
  (add `/Game/Dynamic/Grimics/HiddenBlueprints/BP_GrimicBlueprint.OnInteractedWithGrimicBlueprint` (`self.HiddenActor`) (delegate `OnInteractedWithGrimicBlueprint`))
  (`self.ToggleShownTarget` false))

(event `OnInteractedWithGrimicBlueprint`
  (set `self.IsHidden` false)
  (`self.ToggleShownTarget` true)
  (`ActorComponent.Activate` (`self.NS_Confetti`) false))

(fn `Interact`
  (params (Interacter :type "/Game/Dynamic/FirstPerson/Blueprints/BP_FirstPersonCharacter Object Reference"))
  (returns (result :type Boolean))
  (set `self.Caught` true)
  (`self.IsCaught`)
  (`self.HideGrimic`)
  (return true))

(fn `ToggleInteractionGBP`
  (params (new :type Boolean))
  (set `/Game/Dynamic/Interactables/Blueprints/BaseInteractable.IsInteractable` new (`self.HiddenActor`))
  (return))

(fn `ToggleShownTarget`
  (params (ShowGrimic :type Boolean))
  (bind _hiddenactor (`self.HiddenActor`))
  (bind _hiddenactor_2 (`self.HiddenActor`))
  (if ShowGrimic
    (`self.SetActorHiddenInGame` _hiddenactor true)
    (`self.SetActorEnableCollision` _hiddenactor false)
    ;[1 1 1] Activate This Actor's Meshes
    (for _array_element (`self.K2_GetComponentsByClass` "/Script/Engine.MeshComponent")
      (`SceneComponent.SetHiddenInGame` _array_element false false)
      (`self.SetActorEnableCollision` true))
    (else
      (`self.SetActorHiddenInGame` _hiddenactor_2 false)
      (`self.SetActorEnableCollision` _hiddenactor_2 true)
      ;[1 1 1] Deactivate This Actor's Meshes
      (for _array_element_2 (`self.K2_GetComponentsByClass` "/Script/Engine.MeshComponent")
        (`SceneComponent.SetHiddenInGame` _array_element_2 true false)
        (`self.SetActorEnableCollision` false)))))

(fn `UserConstructionScript`)