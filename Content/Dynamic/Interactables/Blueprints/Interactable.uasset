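; Interactable is a Blueprint interface-style contract for objects that an interacter can use.
; It declares functions to interact, highlight and dehighlight, query whether the object is interactable, display interaction dialogue and play an interaction sound.
; Every function is a stub returning false, so the asset holds no behavior of its own.
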(fn `Dehighlight`
  (params (Interacter :type "/Game/Dynamic/Player/Blueprints/BP_FirstPersonCharacter Object Reference"))
  (returns (result :type Boolean))
  (return false))

(fn `DisplayInteractDialogue`
  (returns (result :type Boolean))
  (return false))

(fn `GetValueIsInteractable`
  (returns (Status :type Boolean))
  (return false))

(fn `Highlight`
  (params (Interacter :type "/Game/Dynamic/Player/Blueprints/BP_FirstPersonCharacter Object Reference"))
  (returns (result :type Boolean))
  (return false))

(fn `Interact`
  (params (Interacter :type "/Game/Dynamic/Player/Blueprints/BP_FirstPersonCharacter Object Reference"))
  (returns (result :type Boolean))
  (return false))

(fn `PlayInteractSound`
  (params (interacter :type "/Game/Dynamic/Player/Blueprints/BP_FirstPersonCharacter Object Reference"))
  (returns (result :type Boolean))
  (return false))