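; Painting interactable that starts its associated level objects whitened and removes the white when the painting interaction event fires.
; On BeginPlay it puts a white overlay material on those objects' static meshes and binds to OnInteractWithPainting.
; That event makes each Grimics actor interactable and plays the Unwhite timeline, driving a shared Material Parameter Collection's Progress.
; Interact only sets UnWhiting, whose lerp logic is disconnected, and ShowGrimics is empty.
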(event `self.ReceiveBeginPlay`
  (`|ExecutionSequence`
    (:`then_0`
      (for _array_element (`self.LevelAssociatedObjects`)
        (for _array_element_2 (`self.K2_GetComponentsByClass` _array_element "/Script/Engine.StaticMeshComponent")
          (`MeshComponent.SetOverlayMaterial` _array_element_2 "/Game/Dynamic/World/materials/MI_WhiteUtrecht.MI_WhiteUtrecht"))))
    (:`then_1`
      (add `self.OnInteractWithPainting` (delegate `Enable Interactables`)))))

(event `Enable Interactables`
  (for _array_element (`self.Grimics`)
    (bind _asbase_interactable (cast `/Game/Dynamic/Interactables/Blueprints/BaseInteractable` _array_element))
    (set `/Game/Dynamic/Interactables/Blueprints/BaseInteractable.IsInteractable` true _asbase_interactable)
    (bind (_direction _unwhite) (`Timeline|Unwhite`)
      (:`Update`
        (`KismetMaterialLibrary.SetScalarParameterValue` "/Game/Dynamic/World/materials/MPC_White1.MPC_White1" "Progress" _unwhite)))))

(fn `Interact`
  (params (Interacter :type "/Game/Dynamic/FirstPerson/Blueprints/BP_FirstPersonCharacter Object Reference"))
  (returns (result :type Boolean))
  (set `self.UnWhiting` true))

(fn `ShowGrimics`)

(fn `UserConstructionScript`)