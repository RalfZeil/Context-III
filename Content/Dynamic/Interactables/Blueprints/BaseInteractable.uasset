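; BaseInteractable is a base actor for interactable objects, providing Highlight, Dehighlight and Interact functions that each take an Interacter.
; Highlight applies a highlight overlay material to every mesh component on the actor, and Dehighlight clears it, with both returning true.
; Interact is a stub that returns false, and the event graph and construction script hold no logic.
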(fn `Dehighlight`
  (params (Interacter :type "/Game/Dynamic/FirstPerson/Blueprints/BP_FirstPersonCharacter Object Reference"))
  (returns (result :type Boolean))
  (for _array_element (`self.K2_GetComponentsByClass` "/Script/Engine.MeshComponent")
    (`MeshComponent.SetOverlayMaterial` _array_element null))
  (return true))

(fn `Highlight`
  (params (Interacter :type "/Game/Dynamic/FirstPerson/Blueprints/BP_FirstPersonCharacter Object Reference"))
  (returns (result :type Boolean))
  (for _array_element (`self.K2_GetComponentsByClass` "/Script/Engine.MeshComponent")
    (`MeshComponent.SetOverlayMaterial` _array_element "/Game/Dynamic/Interactables/Materials/MI_Highlight_Inst.MI_Highlight_Inst"))
  (return true))

(fn `Interact`
  (params (Interacter :type "/Game/Dynamic/FirstPerson/Blueprints/BP_FirstPersonCharacter Object Reference"))
  (returns (result :type Boolean))
  (return false))

(fn `UserConstructionScript`)