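; Base character Blueprint for interactables, providing functions for highlighting, an interactable flag and optional dialogue.
; Highlight applies an overlay material to every mesh component and Dehighlight clears it.
; Interact only reports the flag, which ToggleInteraction sets.
; DisplayInteractDialogue separately sends the dialogue asset, if valid, to the first W_Dialogue widget found by class search.
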(fn `Dehighlight`
  (params (Interacter :type "/Game/Dynamic/FirstPerson/Blueprints/BP_FirstPersonCharacter Object Reference"))
  (returns (result :type Boolean))
  (for _array_element (`self.K2_GetComponentsByClass` "/Script/Engine.MeshComponent")
    (`MeshComponent.SetOverlayMaterial` _array_element null))
  (return true))

(fn `DisplayInteractDialogue`
  (returns (result :type Boolean))
  (`/Engine/EditorBlueprintResources/StandardMacros.IsValid` (`self.OnInteractDialogue`)
    (:`Is Valid`
      (bind _foundwidgets (`WidgetBlueprintLibrary.GetAllWidgetsOfClass` "/Game/Dynamic/UI/W_Dialogue.W_Dialogue_C" false))
      (for _array_element _foundwidgets
        (`/Game/Dynamic/UI/W_Dialogue.SetTextToDisplay` _array_element (`self.OnInteractDialogue`))
        (return true)))
    (:`Is Not Valid`
      (return false))))

(fn `GetValueIsInteractable`
  (returns (Status :type Boolean))
  (return (`self.IsInteractable`)))

(fn `Highlight`
  (params (Interacter :type "/Game/Dynamic/FirstPerson/Blueprints/BP_FirstPersonCharacter Object Reference"))
  (returns (result :type Boolean))
  (for _array_element (`self.K2_GetComponentsByClass` "/Script/Engine.MeshComponent")
    (`MeshComponent.SetOverlayMaterial` _array_element "/Game/Dynamic/Interactables/Materials/MI_Highlight_Inst.MI_Highlight_Inst"))
  (return true))

(fn `Interact`
  (params (Interacter :type "/Game/Dynamic/FirstPerson/Blueprints/BP_FirstPersonCharacter Object Reference"))
  (returns (result :type Boolean))
  (return (`self.IsInteractable`)))

(fn `ToggleInteraction`
  (params (NewState :type Boolean))
  (set `self.IsInteractable` NewState)
  (return))

(fn `UserConstructionScript`)